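; Grappling hook component for BP_Pilot_Master that pulls the pilot toward whatever the fired hook hits.
; FireGrapple spawns a hook projectile and attached cable; a hit zeroes friction and gravity, lowers air control and launches the pilot.
; Tick applies pull force, destroying the hook within range or once a 2D dot product detects overshoot.
; Hook destruction, also triggered by CancelGrapple, removes the cable and restores movement settings and pre-grapple velocity.
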(event EventTick
  (params (DeltaSeconds :type Float%20%28single-precision%29))
  (bind _grapplehook (Variables|ref|GetGrappleHook))
  (bind _returnvalue (Transformation|GetActorLocation _grapplehook))
  (switch Utilities|FlowControl|Switch|SwitchonE_GrappleState (Variables|var|GetGrappleState)
    (:NewEnumerator1
      (Utilities|FlowControl|DoOnce false :!label _label
        (:Completed
          (Audio|PlaySoundatLocation "/Game/Pilot_Master/Blueprints/Blueprint_Mechanics/GrapplingHook_Mechanic/Sounds/Zip_Loop_Cue.Zip_Loop_Cue" (Transformation|GetActorLocation (Variables|ref|GetAs%20BP%20Pilot%20Master)) "0, 0, 0" 1.0 1.0 0.0 0 0 0 0))))
    (:NewEnumerator2
      (Utilities|FlowControl|Sequence
        (:then_0
          (Utilities|FlowControl|DoOnce false :!label _label_2
            (:Completed
              (Utilities|IsValid _grapplehook
                (:Is%20Valid
                  (Audio|PlaySoundatLocation "/Game/Pilot_Master/Blueprints/Blueprint_Mechanics/GrapplingHook_Mechanic/Sounds/Game_Kick_5_Cue.Game_Kick_5_Cue" _returnvalue "0, 0, 0" 1.0 1.0 0.0 0 0 0 0)
                  (Audio|PlaySoundatLocation "/Game/Pilot_Master/Blueprints/Blueprint_Mechanics/GrapplingHook_Mechanic/Sounds/Armor_Break_3_Cue.Armor_Break_3_Cue" _returnvalue "0, 0, 0" 1.0 1.0 0.0 0 0 0 0))))))
        (:then_1
          (Physics|AddForce (Variables|ref|GetAs%20Extended%20Character%20Movement%20Comp) (* (Utilities|ToGrappleHook) (Variables|const|GetGrappleForceSpeed)))
          (if (< (Math|Vector|Distance(Vector) (Transformation|GetActorLocation (Variables|ref|GetGrappleHook)) (Transformation|GetActorLocation (Components|GetOwner))) (Variables|Default|GetAcceptDistance))
            (Actor|DestroyActor (Variables|ref|GetGrappleHook))
            (Utilities|FlowControl|Sequence
              (:then_0
                (goto _label Reset))
              (:then_1
                (goto _label_2 Reset)))
            (elif (< (Math|Vector|DotProduct (Variables|var|GetInitialHookDirection2D) (Utilities|ToGrappleHook2D)) 0.0)
              (Actor|DestroyActor (Variables|ref|GetGrappleHook))
              (Utilities|FlowControl|Sequence
                (:then_0
                  (goto _label Reset))
                (:then_1
                  (goto _label_2 Reset))))))))))

(event EventBeginPlay
  (bind _asbp_pilot_master (Utilities|Casting|CastToBP_Pilot_Master (Components|GetOwner)))
  (Utilities|IsValid _asbp_pilot_master
    (:Is%20Valid
      (bind _output_get (Variables|ref|SetAs%20BP%20Pilot%20Master _asbp_pilot_master))
      (bind _asextended_character_movement_comp (Utilities|Casting|CastToExtendedCharacterMovementComp (Pawn|GetMovementComponent _output_get)))
      (Utilities|IsValid _asextended_character_movement_comp
        (:Is%20Valid
          (Variables|ref|SetAs%20Extended%20Character%20Movement%20Comp _asextended_character_movement_comp))))))

(fn IsinUse?
  (return (Utilities|Select :Index (Variables|var|GetGrappleState) :NewEnumerator0 false :NewEnumerator1 true :NewEnumerator2 true)))

(fn FireGrapple
  (params (TargetLocation :type Vector) (LocalOffset :type Vector))
  (bind _as_bp_pilot_master (Variables|ref|GetAs%20BP%20Pilot%20Master))
  (if (not (CallFunction|IsinUse?))
    (Variables|var|SetGrappleState "NewEnumerator1")
    (LocalVariables|SetFireDirection (Math|Vector|Normalize (- TargetLocation (Utilities|CableStartLocation LocalOffset))))
    (bind _returnvalue (Game|SpawnActorfromClass "/Game/Pilot_Master/Blueprints/Blueprint_Mechanics/GrapplingHook_Mechanic/BP_Grapple_Hook.BP_Grapple_Hook_C" (Math|Transform|MakeTransform (Utilities|CableStartLocation LocalOffset) "-90.000000,0.000000,0.000000" "1.000000,1.000000,1.000000") "Undefined" "MultiplyWithRoot" _as_bp_pilot_master (* (LocalVariables|GetFireDirection) (Variables|const|GetHookSpeed)) _as_bp_pilot_master))
    (bind _output_get (Variables|ref|SetGrappleHook _returnvalue))
    (Collision|BindEventtoOnActorHit _output_get (EventDispatchers|CreateEvent :!event GrappleHit))
    (Game|BindEventtoOnDestroyed (Variables|ref|GetGrappleHook) (EventDispatchers|CreateEvent :!event OnGrappleHookDestroyed))
    (bind _returnvalue_2 (Game|SpawnActorfromClass "/Game/Pilot_Master/Blueprints/Blueprint_Mechanics/GrapplingHook_Mechanic/BP_Hook_Cable.BP_Hook_Cable_C" (Math|Transform|MakeTransform (Utilities|CableStartLocation LocalOffset) (Math|Rotator|MakeRotfromX (LocalVariables|GetFireDirection)) "1.000000,1.000000,1.000000") "Undefined" "MultiplyWithRoot" 0 0))
    (bind _output_get_2 (Variables|ref|SetHookCable _returnvalue_2))
    (Transformation|AttachComponentToComponent _output_get_2 (Variables|/Game/Pilot_Master/Blueprints/FPS_Core/BP_Pilot_Master.BP_Pilot_Master_C|GetGrapplingHookLauncher (Variables|ref|GetAs%20BP%20Pilot%20Master)) "FireGrapple" "KeepWorld" "KeepWorld" "KeepWorld" true)
    (Class|CableComponent|SetAttachEndtoComponent (Variables|/Script/CableComponent.CableActor|GetCableComponent (Variables|ref|GetHookCable)) (Variables|/Game/Pilot_Master/Blueprints/Blueprint_Mechanics/GrapplingHook_Mechanic/BP_Grapple_Hook.BP_Grapple_Hook_C|GetHookMesh (Variables|ref|GetGrappleHook)) "CableAttach")
    (Variables|/Script/CableComponent.CableComponent|SetEndLocation (Variables|/Script/CableComponent.CableActor|GetCableComponent (Variables|ref|GetHookCable)) "0, 0, 0")))

(fn CancelGrapple
  (bind _grapplehook (Variables|ref|GetGrappleHook)
    (:then
      (Actor|DestroyActor _grapplehook))
    (:else)))

(fn GrappleHit
  (params (SelfActor :type Actor%20Object%20Reference) (OtherActor :type Actor%20Object%20Reference) (NormalImpulse :type Vector) (Hit :type Hit%20Result%20Structure%20%28by%20ref%29))
  (bind _as_bp_pilot_master (Variables|ref|GetAs%20BP%20Pilot%20Master))
  (bind _extendedcharactermovementcomponent (Variables|/Script/FPS_Mechanics.ExtendedCharacter|GetExtendedCharacterMovementComponent _as_bp_pilot_master))
  (Variables|var|SetGrappleState "NewEnumerator2")
  (Variables|var|SetVelocityBeforeGrapple (Variables|/Script/Engine.MovementComponent|GetVelocity _extendedcharactermovementcomponent))
  (Variables|/Script/Engine.CharacterMovementComponent|SetGroundFriction _extendedcharactermovementcomponent 0.0)
  (Variables|/Script/Engine.CharacterMovementComponent|SetGravityScale _extendedcharactermovementcomponent 0.0)
  (Variables|/Script/Engine.CharacterMovementComponent|SetAirControl _extendedcharactermovementcomponent 0.2)
  (Variables|/Script/Engine.MovementComponent|SetVelocity _extendedcharactermovementcomponent (* (Utilities|ToGrappleHook) (Variables|const|GetInitialForce)))
  (Variables|var|SetInitialHookDirection2D (Utilities|ToGrappleHook2D))
  (return))

(fn OnGrappleHookDestroyed
  (params (DestroyedActor :type Actor%20Object%20Reference))
  (bind _as_bp_pilot_master (Variables|ref|GetAs%20BP%20Pilot%20Master))
  (bind _extendedcharactermovementcomponent (Variables|/Script/FPS_Mechanics.ExtendedCharacter|GetExtendedCharacterMovementComponent _as_bp_pilot_master))
  (Variables|ref|SetGrappleHook 0)
  (Variables|var|SetGrappleState "NewEnumerator0")
  (Utilities|FlowControl|Sequence
    (:then_0
      (bind _hookcable (Variables|ref|GetHookCable)
        (:then
          (Actor|DestroyActor _hookcable)
          (Variables|ref|SetHookCable 0))
        (:else)))
    (:then_1
      (Variables|/Script/Engine.CharacterMovementComponent|SetGroundFriction _extendedcharactermovementcomponent 1e+01)
      (Variables|/Script/Engine.CharacterMovementComponent|SetGravityScale _extendedcharactermovementcomponent 1.0)
      (Variables|/Script/Engine.CharacterMovementComponent|SetAirControl _extendedcharactermovementcomponent 0.7)
      ;[1 1 1] Reset velocity to value before hooking was started
      (Variables|/Script/Engine.MovementComponent|SetVelocity _extendedcharactermovementcomponent (Variables|var|GetVelocityBeforeGrapple)))))