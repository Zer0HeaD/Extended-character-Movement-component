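; Character movement component that adds sprint, crouch and slide through a four-state machine (walking, sprinting, crouching, sliding).
; Input events and Tick checks drive state changes, which set walk speed and call Crouch/UnCrouch, with a line trace testing headroom.
; Sliding boosts velocity forward and lowers friction and braking.
; A looping timer adds downhill force from the floor normal, caps speed and exits the slide below crouch speed.
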(event Custom|Begin%20Crouch
  (Character|Crouch (Variables|OwnerRef|GetOwner_Character)))

(event Custom|End%20Crouch
  (Variables|Keys|SetCrouchKeyDown false)
  (Character|UnCrouch (Variables|OwnerRef|GetOwner_Character))
  (CallFunction|ResolveMovementState))

(event Custom|Start%20Sprinting
  (Variables|Keys|SetSprintKeyDown true)
  (Utilities|SwitchMovementState
    (:Walking
      _)
    (:Crouching
      _))
  (CallFunction|ResolveMovementState))

(event Custom|Stop%20Sprinting
  (Variables|Keys|SetSprintKeyDown false)
  (Utilities|SwitchMovementState
    (:Sprinting
      (CallFunction|ResolveMovementState))))

(event Custom|Begin%20Slide
  (bind _returnvalue (Utilities|Time|SetTimerbyEvent (delegate Custom|Launch%20Slide) 0.01 true))
  (Variables|Default|SetSlideTimer _returnvalue))

(event Custom|End%20Slide
  (Pawn|Components|CharacterMovement|ClearAccumulatedForces (Variables|OwnerRef|GetMovementComponent))
  (Utilities|Time|ClearandInvalidateTimerbyHandle (Variables|Default|GetSlideTimer)))

(event Custom|Launch%20Slide
  (Physics|AddForce (Variables|OwnerRef|GetMovementComponent) (CallFunction|CalculateFloorInfluence (.Normal (Collision|BreakHitResult (.hitresult (Variables|/Script/Engine.CharacterMovementComponent|GetCurrentFloor (Variables|OwnerRef|GetMovementComponent)))))))
  (Utilities|FlowControl|Sequence
    (:then_0
      (if (> (Math|Vector|VectorLength (Transformation|GetVelocity (Variables|OwnerRef|GetOwner_Character))) (* (Variables|Speeds|GetSprintSpeed) (Variables|Default|GetSlideMultiplier)))
        (Variables|/Script/Engine.MovementComponent|SetVelocity (Variables|OwnerRef|GetMovementComponent) (* (Math|Vector|Normalize (Transformation|GetVelocity (Variables|OwnerRef|GetOwner_Character))) (* (Variables|Speeds|GetSprintSpeed) (Variables|Default|GetSlideMultiplier))))))
    (:then_1
      (if (< (Math|Vector|VectorLength (Transformation|GetVelocity (Variables|OwnerRef|GetOwner_Character))) (Variables|Speeds|GetCrouchSpeed))
        (CallFunction|ResolveMovementState)
        (CallFunction|EndSlide)))))

(event Custom|Toggle%20Crouch
  (if (and (Variables|/Script/Engine.Character|GetbIsCrouched (Variables|OwnerRef|GetOwner_Character)) (not (AI|Components|NavMovement|IsFalling (Variables|OwnerRef|GetMovementComponent))))
    (CallFunction|EndCrouch)
    (else
      (Variables|Keys|SetCrouchKeyDown true)
      (Utilities|SwitchMovementState
        (:Walking
          (CallFunction|SetMovementState "NewEnumerator2"))
        (:Sprinting
          (CallFunction|SetMovementState "NewEnumerator3"))))))

(event EventBeginPlay
  (Utilities|FlowControl|Sequence
    (:then_0
      (|SetRefstocharacterandmovementcomponent))
    (:then_1
      (Variables|Movement|SetStandingCapsuleHalfHeight (Components|Capsule|GetScaledCapsuleHalfHeight (Variables|/Script/Engine.Character|GetCapsuleComponent (Variables|OwnerRef|GetOwner_Character))))
      (Variables|Movement|SetStandingCamerazOffset 51.0) ; Relative Location of Z Camera. Hardcoded
    )))

(event EventTick
  (params (DeltaSeconds :type Float%20%28single-precision%29))
  (Development|PrintText (Utilities|Text|FormatText "Crouch state: {isCouch}" (Utilities|Text|ToText(Boolean) (AI|Components|NavMovement|IsCrouching (Variables|OwnerRef|GetMovementComponent)))) true true "(R=0.000000,G=0.660000,B=1.000000,A=1.000000)" 0.0 "1frame")
  (Utilities|SwitchMovementState
    (:Sprinting
      (if (AI|Components|NavMovement|IsFalling (Variables|OwnerRef|GetMovementComponent))
        (Variables|Keys|SetSprintKeyDown false)
        (Utilities|SwitchMovementState
          (:Sprinting
            (CallFunction|ResolveMovementState)))))
    (:Crouching
      (if (CallFunction|CanStand)
        (CallFunction|ResolveMovementState)))
    (:Sliding
      (if (AI|Components|NavMovement|IsFalling (Variables|OwnerRef|GetMovementComponent))
        (CallFunction|EndCrouch)))))

(fn SetMovementState
  (params (NewMovementState :type E_Slide_MovementStates%20Enum :default "NewEnumerator0"))
  (if (Utilities|Enum|NotEqual(Enum) NewMovementState (Variables|Movement|GetMovementState))
    (LocalVariables|SetPrevMovementState%28Local%29 (Variables|Movement|GetMovementState))
    (Variables|Movement|SetMovementState NewMovementState)
    (CallFunction|OnMovementStateChanged (LocalVariables|GetPrevMovementState%28Local%29))
    (Utilities|SwitchMovementState
      (:Walking
        (CallFunction|EndCrouch :!label _label))
      (:Sprinting
        (goto _label))
      (:Crouching
        (CallFunction|BeginCrouch))
      (:Sliding
        (CallFunction|BeginCrouch)
        (CallFunction|BeginSlide)))))

(fn ResolveMovementState
  (CallFunction|SetMovementState (select (CallFunction|CanSprint) "NewEnumerator1" (select (CallFunction|CanStand) "NewEnumerator0" "NewEnumerator2"))))

(fn OnMovementStateChanged
  (params (PrevMovementState :type E_Slide_MovementStates%20Enum :default "NewEnumerator0"))
  (bind _movementcomponent (Variables|OwnerRef|GetMovementComponent))
  (Utilities|FlowControl|Sequence
    (:then_0
      (Variables|/Script/Engine.CharacterMovementComponent|SetMaxWalkSpeed (Variables|OwnerRef|GetMovementComponent) (Utilities|Select :Index (Variables|Movement|GetMovementState) :NewEnumerator0 (Variables|Speeds|GetWalkSpeed) :NewEnumerator1 (Variables|Speeds|GetSprintSpeed) :NewEnumerator2 (Variables|Speeds|GetCrouchSpeed) :NewEnumerator3 0.0)))
    (:then_1
      (switch Utilities|FlowControl|Switch|SwitchonE_Slide_MovementStates PrevMovementState
        (:NewEnumerator3
          (Variables|/Script/Engine.CharacterMovementComponent|SetGroundFriction _movementcomponent 8.0)
          (Variables|/Script/Engine.CharacterMovementComponent|SetBrakingDecelerationWalking _movementcomponent 2048.0))))
    (:then_2
      (Utilities|SwitchMovementState
        (:Sliding
          (Variables|/Script/Engine.MovementComponent|SetVelocity (Variables|OwnerRef|GetMovementComponent) (* (Transformation|GetActorForwardVector (Variables|OwnerRef|GetOwner_Character)) (* (Variables|Speeds|GetSprintSpeed) (Variables|Default|GetSlideMultiplier))))
          (Variables|/Script/Engine.CharacterMovementComponent|SetGroundFriction (Variables|OwnerRef|GetMovementComponent) 0.2)
          (Variables|/Script/Engine.CharacterMovementComponent|SetBrakingDecelerationWalking (Variables|OwnerRef|GetMovementComponent) 5e+02))))))

(fn CalculateFloorInfluence
  (params (FloorNormal :type Vector))
  (if (Utilities|Operators|EqualEqual FloorNormal (Math|Vector|VectorUp) 0.0001)
    (return "0, 0, 0")
    (else
      (return (* (Math|Vector|Normalize (Math|Vector|CrossProduct FloorNormal (Math|Vector|CrossProduct FloorNormal (Math|Vector|VectorUp)))) (* (Math|Float|Clamp(Float) (- 1.0 (Math|Vector|DotProduct FloorNormal (Math|Vector|VectorUp)))) 1e+06))))))

(fn CanSprint
  (if (Variables|Keys|GetSprintKeyDown)
    (return (and (CallFunction|CanStand) (not (AI|Components|NavMovement|IsFalling (Variables|OwnerRef|GetMovementComponent)))))
    (else
      (return false))))

(fn CanStand
  (bind _owner_character (Variables|OwnerRef|GetOwner_Character))
  (bind _returnvalue (Transformation|GetActorLocation _owner_character))
  (bind _capsulecomponent (Variables|/Script/Engine.Character|GetCapsuleComponent _owner_character))
  (bind _returnvalue_2 (Components|Capsule|GetScaledCapsuleHalfHeight _capsulecomponent))
  (bind _returnvalue_3 (- _returnvalue (Math|Vector|MakeVector 0.0 0.0 _returnvalue_2)))
  (if (Variables|/Script/Engine.Character|GetbIsCrouched (Variables|OwnerRef|GetOwner_Character))
    (return false)
    (else
      (bind _returnvalue_4 (Collision|LineTraceByChannel _returnvalue_3 (+ _returnvalue_3 (Math|Vector|MakeVector 0.0 0.0 (* (Variables|Movement|GetStandingCapsuleHalfHeight) 2.0))) "TraceTypeQuery1" false 0 "None"))
      (return (not _returnvalue_4)))))